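; AI controller that drives a wheeled vehicle through racing waypoints, optionally looping.
; A timed update follows navigation paths to each waypoint, detects opponents ahead by overlap and can line-trace four sides to override inputs.
; Steering adds opponent avoidance, while throttle and braking follow waypoint speed, curve anticipation and the car ahead, reversing when stuck.
; Inputs go to Chaos vehicle movement or, with CustomEvents, to pawn interface messages.
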(event `/Game/Blueprints/Data/Interfaces/BPI_EZRacing.Initialize`
  (params (StartDelay :type "Float (double-precision)") (StartingIndex :type Integer) (LoopPath :type Boolean) (Waypoints :type "Array of /Game/Blueprints/Actors/BP_EZRacingWaypoint Object Reference (by ref)") (OpponentClasses :type "Array of Actor Class Reference (by ref)"))
  ;[0 0 0] AI
  ;;[1 1 1] Initialize AI
  (set `self.Index` StartingIndex)
  (set `self.LoopPath` LoopPath)
  (set `self.Waypoints` Waypoints)
  (set `self.Opponents` OpponentClasses)
  (`self.Begin` StartDelay))

(event `Update`
  (bind _controlledpawn (`self.ControlledPawn`))
  (bind _desiredspeed (`self.DesiredSpeed`))
  (bind _controlledpawn_2 (`self.ControlledPawn`))
  (bind _maxsteer (`self.MaxSteer`))
  (bind _wvmc (`self.WVMC`))
  (bind _wvmc_2 (`self.WVMC`))
  (bind _controlledpawn_3 (`self.ControlledPawn`))
  (bind _returnvalue (`ChaosVehicleMovementComponent.GetForwardSpeed` (`self.WVMC`)))
  (bind _returnvalue_2 (`KismetMathLibrary.MapRangeClamped` 0.0 (+ _desiredspeed 15.0) (+ _desiredspeed 50.0) 0.0 0.5))
  (bind _returnvalue_3 (< (`KismetMathLibrary.VSize` (`self.GetVelocity` (`self.ControlledPawn`))) 10.0))
  (bind _returnvalue_4 (`KismetMathLibrary.DegAcos` (`KismetMathLibrary.Dot_VectorVector` (`KismetMathLibrary.Normal` (- (`self.TargetLoc`) (`self.K2_GetActorLocation` _controlledpawn_2))) (`self.GetActorForwardVector` _controlledpawn_2))))
  (bind _returnvalue_5 (> _returnvalue_4 _maxsteer))
  (bind _returnvalue_6 (`KismetMathLibrary.MapRangeClamped` (- _returnvalue_4 _maxsteer) 5.0 50.0 0.9 0.5))
  (bind _returnvalue_7 (`KismetMathLibrary.SelectFloat` 1.0 0.0 (> _returnvalue_4 (+ _maxsteer 20.0))))
  ;[0 0 0] AI
  ;;[1 1 1] Update AI
  (`self.FindTarget`)
  (`self.Detect Opponents`)
  (`self.CalcAvoidance`)
  (`self.Steering`)
  (set `self.DesiredSpeed` (`self.Get DesiredSpeed`))
  (if (`self.Reverse`)
    (if (`self.CustomEvents`)
      (message `/Game/Blueprints/Data/Interfaces/BPI_CustomEvents.Set Steering Input` _controlledpawn_3 0.0)
      (message `/Game/Blueprints/Data/Interfaces/BPI_CustomEvents.Set Throttle Input` _controlledpawn_3 -1.0)
      (else
        (`ChaosVehicleMovementComponent.SetSteeringInput` _wvmc_2 0.0)
        (`ChaosVehicleMovementComponent.SetThrottleInput` _wvmc_2 -1.0)))
    (`self.CalcDistance` :!label _label)
    (elif _returnvalue_3
      (`KismetSystemLibrary.Delay` 2.0)
      (if _returnvalue_3
        (set `self.Reverse` true)
        (`KismetSystemLibrary.Delay` 1.0)
        (set `self.Reverse` false)
        (else
          (if (`self.CustomEvents`) :!label _label_2
            (if (> (* (`KismetMathLibrary.VSize` (`self.GetVelocity` (`self.ControlledPawn`))) 1.0) (+ (`self.DesiredSpeed`) 1.0))
              (message `/Game/Blueprints/Data/Interfaces/BPI_CustomEvents.Set Throttle Input` (`self.ControlledPawn`) 0.0)
              (if (> (* (`KismetMathLibrary.VSize` (`self.GetVelocity` (`self.ControlledPawn`))) 1.0) (`/Game/Blueprints/Actors/BP_EZRacingWaypoint.WaypointSpeed` (`self.TargetWaypoint`)))
                (message `/Game/Blueprints/Data/Interfaces/BPI_CustomEvents.SetBrakeInput` (`self.ControlledPawn`) _returnvalue_2)
                (goto _label)
                (else
                  (goto _label)))
              (else
                (message `/Game/Blueprints/Data/Interfaces/BPI_CustomEvents.Set Throttle Input` _controlledpawn (`KismetMathLibrary.SelectFloat` (`self.ThrottleOverride`) (`KismetMathLibrary.SelectFloat` _returnvalue_6 (`KismetMathLibrary.SelectFloat` 0.0 1.0 (> (* (`KismetMathLibrary.VSize` (`self.GetVelocity` (`self.ControlledPawn`))) 1.0) (`/Game/Blueprints/Actors/BP_EZRacingWaypoint.WaypointSpeed` (`self.TargetWaypoint`)))) _returnvalue_5) (`self.OverrideThrottle`)))
                (message `/Game/Blueprints/Data/Interfaces/BPI_CustomEvents.SetBrakeInput` _controlledpawn _returnvalue_7)
                (goto _label)))
            (elif (> _returnvalue (+ (`self.DesiredSpeed`) 1.0))
              (`ChaosVehicleMovementComponent.SetThrottleInput` (`self.WVMC`) 0.0)
              (if (> _returnvalue (+ (`self.DesiredSpeed`) 10.0))
                (`ChaosVehicleMovementComponent.SetBrakeInput` (`self.WVMC`) _returnvalue_2)
                (goto _label)
                (else
                  (goto _label)))
              (else
                (`ChaosVehicleMovementComponent.SetThrottleInput` _wvmc (`KismetMathLibrary.SelectFloat` (`self.ThrottleOverride`) (`KismetMathLibrary.SelectFloat` _returnvalue_6 (`KismetMathLibrary.SelectFloat` 0.0 1.0 (> (`ChaosVehicleMovementComponent.GetForwardSpeed` (`self.WVMC`)) (`/Game/Blueprints/Actors/BP_EZRacingWaypoint.WaypointSpeed` (`self.TargetWaypoint`)))) _returnvalue_5) (`self.OverrideThrottle`)))
                (`ChaosVehicleMovementComponent.SetBrakeInput` _wvmc _returnvalue_7)
                (goto _label))))))
      (else
        (goto _label_2)))))

(event `Begin`
  (params (Delay :type "Float (double-precision)"))
  ;[0 0 0] AI
  ;;[1 1 1] Initialize AI
  (`KismetSystemLibrary.Delay` Delay)
  (bind _output_get (set `self.ControlledPawn` (`self.K2_GetPawn`)))
  (if (`self.CustomEvents`)
    (`KismetSystemLibrary.Delay` 0.01 :!label _label_3)
    (bind _output_get_2 (set `self.TargetWaypoint` (`|GetArrayItem` (`self.Waypoints`) (`self.Index`))))
    (`/Engine/EditorBlueprintResources/StandardMacros.IsValid` _output_get_2
      (:`Is Valid`
        (if (`self.CustomEvents`)
          (message `/Game/Blueprints/Data/Interfaces/BPI_CustomEvents.Set Throttle Input` (`self.ControlledPawn`) 1.0)
          (else
            (`ChaosVehicleMovementComponent.SetThrottleInput` (`self.WVMC`) 1.0)))
        (`KismetSystemLibrary.K2_SetTimerDelegate` (delegate `Update`) (`self.UpdateFreq`) true 0.1))
      (:`Is Not Valid`
        (`KismetSystemLibrary.PrintString` "Invalid Waypoint Index!")))
    (else
      (bind _aschaos_wheeled_vehicle_movement_component (cast `ChaosWheeledVehicleMovementComponent` (`Pawn.GetMovementComponent` _output_get))
        (:`then`
          (set `self.WVMC` _aschaos_wheeled_vehicle_movement_component)
          (goto _label_3))
        (:`CastFailed`
          (`KismetSystemLibrary.PrintString` "NO WHEELED VEHICLE MOVEMENT COMPONENT FOUND! Enable and Add Custom Events or Add Wheeled Vehicle Movement Component." true true (struct :`R` 1.0 :`A` 1.0) 100.0))))))

(fn `CalcAvoidance`
  (locals (Ahead :type Boolean :default false) (Right :type Boolean :default false) (Left :type Boolean :default false) (Behind :type Boolean :default false))
  (bind _right (`local.Right`))
  (bind _behind (`local.Behind`))
  (bind _controlledpawn (`self.ControlledPawn`))
  (bind _returnvalue (`self.GetActorForwardVector` _controlledpawn))
  (bind _origin (`self.GetActorBounds` _controlledpawn true false))
  (bind _returnvalue_2 (`self.GetActorRightVector` _controlledpawn))
  (bind _array (`|MakeArray` (`self.ControlledPawn`) :!type "Actor Object Reference"))
  ;[1 1 1] Start
  (if (`self.TraceAvoidance`)
    ;[0 0 0] Trace Ahead, Behind, Front, and Left
    ;;[1 1 1] Trace Ahead
    (bind (_outhit _returnvalue_3) (`KismetSystemLibrary.LineTraceSingle` _origin (+ (* _returnvalue (`self.TraceAvoidanceRadius`)) _origin) "TraceTypeQuery1" false _array)) ; Ahead
    (set `local.Ahead` _returnvalue_3)
    ;;[1 1 1] Trace Behind
    (bind (_outhit_2 _returnvalue_4) (`KismetSystemLibrary.LineTraceSingle` _origin (+ (* (* _returnvalue -1.0) (`self.TraceAvoidanceRadius`)) _origin) "TraceTypeQuery1" false _array)) ; Behind
    (set `local.Behind` _returnvalue_4)
    ;;[1 1 1] Trace Right
    (bind (_outhit_3 _returnvalue_5) (`KismetSystemLibrary.LineTraceSingle` _origin (+ (* _returnvalue_2 (`self.TraceAvoidanceRadius`)) _origin) "TraceTypeQuery1" false _array)) ; Right
    (set `local.Right` _returnvalue_5)
    ;;[1 1 1] Trace Left
    (bind (_outhit_4 _returnvalue_6) (`KismetSystemLibrary.LineTraceSingle` _origin (+ (* (* _returnvalue_2 -1.0) (`self.TraceAvoidanceRadius`)) _origin) "TraceTypeQuery1" false _array)) ; Left
    (bind _output_get (set `local.Left` _returnvalue_6))
    ;[0 0 0] Override as Necessary
    ;;[1 1 1] Effect Steering
    (if (not (`KismetMathLibrary.BooleanNAND` _output_get _right))
      (set `self.OverrideSteering` true)
      (if (or (not (`local.Ahead`)) (and _right (`local.Left`)))
        (set `self.SteeringOverride` 0.0)
        (elif _right
          (set `self.SteeringOverride` -1.0)
          (else
            (set `self.SteeringOverride` 1.0)))))
    ;;[1 1 1] Effect Throttle
    (if (not (`KismetMathLibrary.BooleanNAND` (`local.Ahead`) (`local.Behind`)))
      (set `self.OverrideThrottle` true)
      (if (and (`local.Ahead`) _behind)
        (set `self.ThrottleOverride` 0.5)
        (elif _behind
          (set `self.ThrottleOverride` 1.0)
          (else
            (set `self.ThrottleOverride` 0.0)))))
    (return)
    (else
      (return))))

(fn `CalcDistance`
  (bind _targetwaypoint (`self.TargetWaypoint`))
  (bind _waypoints (`self.Waypoints`))
  (bind _index (`self.Index`))
  (if (not (and (> (`KismetMathLibrary.VSize` (- (`self.K2_GetActorLocation` (`self.ControlledPawn`)) (`self.K2_GetActorLocation` _targetwaypoint))) (`/Game/Blueprints/Actors/BP_EZRacingWaypoint.AcceptanceRadius` _targetwaypoint)) (`KismetSystemLibrary.IsValid` (`self.TargetWaypoint`))))
    ;[1 1 1] Switch Waypoints
    (bind _output_get (set `self.Index` (`KismetMathLibrary.SelectInt` 0 (+ _index 1) (and (== (`KismetArrayLibrary.Array_LastIndex` _waypoints) _index) (`self.LoopPath`)))))
    (set `self.TargetWaypoint` (`|GetArrayItem` _waypoints _output_get)))
  (return))

(fn `CalcSteerAvoidance`
  (returns (ReturnValue :type "Float (double-precision)"))
  (bind _detectedopponents (`self.DetectedOpponents`))
  (bind (_opponent _distance _angle) (break `/Game/Blueprints/Data/Struc/S_EZRacingOpponent` (`|GetArrayItem` _detectedopponents (`self.Closest Opponent Index`))))
  (bind _returnvalue (`KismetMathLibrary.Abs` _angle))
  (bind _returnvalue_2 (* (* (`KismetMathLibrary.MapRangeClamped` _returnvalue 5.0 15.0 (`KismetMathLibrary.MapRangeClamped` _distance (`KismetMathLibrary.Lerp` 700.0 400.0 (`KismetMathLibrary.MapRangeClamped` _returnvalue 5.0 15.0 0.0 1.0)) 1000.0 45.0 15.0) (`KismetMathLibrary.MapRangeClamped` _distance 300.0 700.0 5.0)) (`KismetMathLibrary.SignOfFloat` _angle)) -1.0))
  (if (`KismetArrayLibrary.Array_IsValidIndex` _detectedopponents)
    (return (* (`KismetMathLibrary.MapRangeClamped` (`KismetMathLibrary.Abs` _returnvalue_2) 0.0 45.0 0.0 1.0) (`KismetMathLibrary.SignOfFloat` _returnvalue_2)))
    (else
      (return 0.0))))

(fn `Detect Opponents`
  (locals (TempOpponent :type "Array of Actor Object Reference") (TempShortestDistance :type "Float (double-precision)" :default 2000.0) (TempClosestOpponentIndex :type Integer :default 0) (TempMostInFrontAngle :type "Float (double-precision)" :default 90.0) (TempMostInFrontOpponentIndex :type Integer))
  (bind _tempopponent (`local.TempOpponent`))
  (bind _controlledpawn (`self.ControlledPawn`))
  (bind _detectedopponents (`self.DetectedOpponents`))
  (bind _returnvalue (`self.GetActorForwardVector` _controlledpawn))
  ;[1 1 1] Get Overlapping Actors in Opponent Classess
  (`KismetArrayLibrary.Array_Clear` (`self.DetectedOpponents`))
  (for _array_element (`self.Opponents`)
    (`KismetArrayLibrary.Array_Append` (`local.TempOpponent`) (`PrimitiveComponent.GetOverlappingActors` (`self.Collision`) _array_element)))
  ;[1 1 1] Make Opponent Data
  (if (`KismetArrayLibrary.Array_IsValidIndex` _tempopponent)
    (for _array_element_2 _tempopponent
      (bind _returnvalue_2 (- (`self.K2_GetActorLocation` _array_element_2) (`self.K2_GetActorLocation` _controlledpawn)))
      (bind _returnvalue_3 (`KismetMathLibrary.Normal` _returnvalue_2))
      (bind _returnvalue_4 (`KismetMathLibrary.DegAcos` (`KismetMathLibrary.Dot_VectorVector` _returnvalue_3 _returnvalue)))
      (if (< _returnvalue_4 90.0)
        (bind (_returnvalue_x _returnvalue_y _returnvalue_z) (`KismetMathLibrary.BreakVector` (`KismetMathLibrary.Cross_VectorVector` (`KismetMathLibrary.Normal` _returnvalue) _returnvalue_3)))
        (`KismetArrayLibrary.Array_Add` (`self.DetectedOpponents`) (make `/Game/Blueprints/Data/Struc/S_EZRacingOpponent` _array_element_2 (`KismetMathLibrary.VSize` _returnvalue_2) (* _returnvalue_4 _returnvalue_z)))))
    ;[1 1 1] Get Closest Opponent
    (if (`KismetArrayLibrary.Array_IsValidIndex` _detectedopponents)
      (for (_array_element_3 _array_index) _detectedopponents
        (bind (_opponent _distance) (break `/Game/Blueprints/Data/Struc/S_EZRacingOpponent` _array_element_3))
        (if (< _distance (`local.TempShortestDistance`))
          (set `local.TempClosestOpponentIndex` _array_index)
          (set `local.TempShortestDistance` _distance)))
      (set `self.Closest Opponent Index` (`local.TempClosestOpponentIndex`))
      ;[1 1 1] Get Most In Front Opponent
      (for (_array_element_4 _array_index_2) (`self.DetectedOpponents`)
        (bind _returnvalue_5 (`KismetMathLibrary.Abs` (`.Angle_7_34E1D1424DEA801B64E36EA4E701EF50` (break `/Game/Blueprints/Data/Struc/S_EZRacingOpponent` _array_element_4))))
        (if (< _returnvalue_5 (`local.TempMostInFrontAngle`))
          (set `local.TempMostInFrontOpponentIndex` _array_index_2)
          (set `local.TempMostInFrontAngle` _returnvalue_5)))
      (set `self.MostInFrontOpponentIndex` (`local.TempMostInFrontOpponentIndex`))
      (return)
      (else
        (return)))
    (else
      (return))))

(fn `FindTarget`
  (bind _controlledpawn (`self.ControlledPawn`))
  (bind _returnvalue (`NavigationSystemV1.FindPathToLocationSynchronously` (`self.K2_GetActorLocation` _controlledpawn) (`self.K2_GetActorLocation` (`self.TargetWaypoint`)) _controlledpawn null)) ; Use Navigation Volume for navigation.
  (set `self.TargetLoc` (`|GetArrayItem` (`NavigationPath.PathPoints` _returnvalue) 1))
  (return))

(fn `Get DesiredSpeed`
  (returns (DesiredSpeed :type "Float (double-precision)"))
  (bind _detectedopponents (`self.DetectedOpponents`))
  (bind _waypointspeed (`/Game/Blueprints/Actors/BP_EZRacingWaypoint.WaypointSpeed` (`self.TargetWaypoint`)))
  (bind (_opponent _distance _angle) (break `/Game/Blueprints/Data/Struc/S_EZRacingOpponent` (`|GetArrayItem` _detectedopponents (`self.MostInFrontOpponentIndex`))))
  (bind _returnvalue (- _waypointspeed (`self.MaxSpeedDifference`)))
  (bind _returnvalue_2 (`KismetMathLibrary.MapRangeClamped` (`KismetMathLibrary.Abs` (`self.GetCurveAnticipation`)) 4.0 15.0 _waypointspeed _returnvalue))
  (if (`KismetArrayLibrary.Array_IsValidIndex` _detectedopponents)
    (return (`KismetMathLibrary.FClamp` _returnvalue_2 _returnvalue (`KismetMathLibrary.Lerp` _waypointspeed (`KismetMathLibrary.Lerp` (* (`KismetMathLibrary.VSize` (`self.GetVelocity` _opponent)) 0.0036) _waypointspeed (`KismetMathLibrary.MapRangeClamped` _distance 160.0 250.0 0.0 1.0)) (`KismetMathLibrary.MapRangeClamped` (`KismetMathLibrary.Abs` _angle) 5.0 15.0 1.0))))
    (else
      (return _returnvalue_2))))

(fn `GetCurveAnticipation`
  (returns (ReturnValue :type "Float (double-precision)"))
  (locals (GreaterThanDesiredSpeed :type Boolean :default false))
  (bind _waypoints (`self.Waypoints`))
  (bind _returnvalue (+ (`self.Index`) 1))
  (bind (_returnvalue_roll _returnvalue_pitch _returnvalue_yaw) (`KismetMathLibrary.BreakRotator` (`KismetMathLibrary.ComposeRotators` (`KismetMathLibrary.NegateRotator` (`KismetMathLibrary.ComposeRotators` (`KismetMathLibrary.MakeRotator` 0.0 0.0 (* (`self.GetSteeringAngle`) (`KismetMathLibrary.SelectFloat` -1.0 1.0 (`local.GreaterThanDesiredSpeed`)))) (`self.K2_GetActorRotation` (`self.ControlledPawn`)))) (`KismetMathLibrary.FindLookAtRotation` (`self.TargetLoc`) (`self.K2_GetActorLocation` (`|GetArrayItem` _waypoints _returnvalue))))))
  (if (`self.CustomEvents`)
    (set `local.GreaterThanDesiredSpeed` (> (* (`KismetMathLibrary.VSize` (`self.GetVelocity` (`self.ControlledPawn`))) 1.0) (`/Game/Blueprints/Actors/BP_EZRacingWaypoint.WaypointSpeed` (`self.TargetWaypoint`))))
    (else
      (set `local.GreaterThanDesiredSpeed` (> (`ChaosVehicleMovementComponent.GetForwardSpeed` (`self.WVMC`)) (`/Game/Blueprints/Actors/BP_EZRacingWaypoint.WaypointSpeed` (`self.TargetWaypoint`))))))
  (if (and (`KismetArrayLibrary.Array_IsValidIndex` _waypoints _returnvalue) (`KismetArrayLibrary.Array_IsNotEmpty` _waypoints))
    (return _returnvalue_yaw)
    (else
      (return 0.0))))

(fn `GetSteeringAngle`
  (returns (SteerAngle :type "Float (double-precision)"))
  (locals (TempAngles :type "Array of Float (double-precision)") (TempSum :type "Float (double-precision)"))
  (bind _tempangles (`local.TempAngles`))
  (if (`self.CustomEvents`)
    (bind _steeringangle (message `/Game/Blueprints/Data/Interfaces/BPI_CustomEvents.GetSteeringAngle` (`self.ControlledPawn`)))
    (return _steeringangle)
    (else
      (for _array_element (`ChaosWheeledVehicleMovementComponent.Wheels` (`self.WVMC`))
        (bind _returnvalue (`ChaosVehicleWheel.GetSteerAngle` _array_element))
        (if (!= _returnvalue 0.0)
          (`KismetArrayLibrary.Array_Add` (`local.TempAngles`) _returnvalue)))
      (if (`KismetArrayLibrary.Array_IsValidIndex` _tempangles)
        (for _array_element_2 _tempangles
          (set `local.TempSum` (+ _array_element_2 (`local.TempSum`))))
        (return (/ (`local.TempSum`) (`KismetMathLibrary.Conv_IntToDouble` (`KismetArrayLibrary.Array_Length` _tempangles))))
        (else
          (return 0.0))))))

(fn `Steering`
  (bind _controlledpawn (`self.ControlledPawn`))
  (bind _controlledpawn_2 (`self.ControlledPawn`))
  (bind _controlledpawn_3 (`self.ControlledPawn`))
  (bind _returnvalue (`KismetMathLibrary.SelectFloat` (`self.SteeringOverride`) (+ (`KismetMathLibrary.SelectFloat` 0.0 (`KismetMathLibrary.SelectFloat` 1.0 -1.0 (< (`KismetMathLibrary.DegAcos` (`KismetMathLibrary.Dot_VectorVector` (`KismetMathLibrary.Normal` (- (`self.TargetLoc`) (`self.K2_GetActorLocation` _controlledpawn_2))) (`self.GetActorRightVector` _controlledpawn_2))) (`KismetMathLibrary.DegAcos` (`KismetMathLibrary.Dot_VectorVector` (`KismetMathLibrary.Normal` (- (`self.TargetLoc`) (`self.K2_GetActorLocation` _controlledpawn_3))) (* (`self.GetActorRightVector` _controlledpawn_3) -1.0))))) (< (`KismetMathLibrary.DegAcos` (`KismetMathLibrary.Dot_VectorVector` (`KismetMathLibrary.Normal` (- (`self.TargetLoc`) (`self.K2_GetActorLocation` _controlledpawn))) (`self.GetActorForwardVector` _controlledpawn))) 10.0)) (`self.CalcSteerAvoidance`)) (`self.OverrideSteering`)))
  (if (`self.CustomEvents`)
    (message `/Game/Blueprints/Data/Interfaces/BPI_CustomEvents.Set Steering Input` (`self.ControlledPawn`) _returnvalue)
    (else
      (`ChaosVehicleMovementComponent.SetSteeringInput` (`self.WVMC`) _returnvalue)))
  (return))

(fn `UserConstructionScript`)