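; Simple AI controller for hover cars, built to drive a BP_VehicleMaster pawn along its AITrack spline.
; Start_Race spawns an invisible target mesh once and caches the pawn and track.
; The movement logic advances that target while the car is near, steers by yaw toward it and adds an upward impulse when stuck.
; That movement chain is disconnected from Tick, so it never runs as wired.
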(event `Start_Race`
  (`/Engine/EditorBlueprintResources/StandardMacros.DoOnce` false
    (:`Completed`
      ;[0 1 0.2449] Spawn Target Actor
      (bind _returnvalue (`|SpawnActorFromClass` "/Script/Engine.StaticMeshActor" (`KismetMathLibrary.MakeTransform` (0.0 0.0 0.0) (struct) (10.0 10.0 1000.0)) "Undefined" "OverrideRootScale" null null))
      (bind _staticmeshcomponent (`StaticMeshActor.StaticMeshComponent` _returnvalue))
      (`SceneComponent.SetVisibility` _staticmeshcomponent false false)
      (`StaticMeshActor.SetMobility` _returnvalue "Movable")
      (`PrimitiveComponent.SetCollisionEnabled` _staticmeshcomponent "NoCollision")
      (set `self.TargetMesh` _returnvalue)
      (`StaticMeshComponent.SetStaticMesh` (`StaticMeshActor.StaticMeshComponent` _returnvalue) "/Game/GameContent/Particles/JetEngine/Meshes/SM_exhaust.SM_exhaust")
      (bind _asbp_hover_car (cast `/Game/Blueprints/BP_VehicleMaster` (`self.K2_GetPawn`)))
      (bind _output_get (set `self.BP_Hover_Car` _asbp_hover_car))
      (set `self.AI_Track` (`/Game/Blueprints/BP_VehicleMaster.AI_Track` _output_get)))))

(event `self.ReceiveTick`
  (params (DeltaSeconds :type "Float (single-precision)"))
  ;[0 1 0.2449] Calculate Movement
)

(fn `UserConstructionScript`)