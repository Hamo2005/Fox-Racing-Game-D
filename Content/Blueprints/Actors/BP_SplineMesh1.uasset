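; Actor that tiles a static mesh along its spline, building the spline mesh components in the construction script.
; Section length comes from the mesh's X bounds, a length offset and scale, optionally rounded to fit the spline length via ConsistentMeshSizes.
; Each section takes positions and tangents from spline distances, with tangent length clamped to the section length, and applies a configurable collision setting.
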(fn `UserConstructionScript`
  (bind _eachsectionlength (`self.EachSectionLength`))
  (bind _distancestart (`self.DistanceStart`))
  (bind _distanceend (`self.DistanceEnd`))
  (bind _eachsectionlength_2 (`self.EachSectionLength`))
  (bind _spline (`self.Spline`))
  (bind _returnvalue (`SplineComponent.GetSplineLength` (`self.Spline`)))
  (bind (_returnvalue_min _returnvalue_max) (break `Box` (`StaticMesh.GetBoundingBox` (`self.StaticMesh`))))
  (`|ExecutionSequence`
    (:`then_0`
      ;[1 1 1] Define section length
      (bind _output_get (set `self.MeshBoundSize` (- _returnvalue_max _returnvalue_min)))
      (bind _returnvalue_2 (* (`self.MeshScale`) (+ (.x _output_get) (`self.MeshLengthAdd`))))
      (set `self.EachSectionLength` (`KismetMathLibrary.Lerp` _returnvalue_2 (`KismetMathLibrary.Conv_IntToDouble` (`KismetMathLibrary.FFloor` (/ _returnvalue (`KismetMathLibrary.Conv_IntToDouble` (`KismetMathLibrary.FFloor` (/ _returnvalue _returnvalue_2)))))) (`KismetMathLibrary.Conv_BoolToDouble` (`self.ConsistentMeshSizes`)))))
    (:`then_1`
      ;[1 1 1] Create Spline Mesh
      (bind _output_get_2 (set `self.NumberOfSections` (`.ReturnValue` (`KismetMathLibrary.FMod` (`SplineComponent.GetSplineLength` (`self.Spline`)) _eachsectionlength_2))))
      (for _index (range (+ (- _output_get_2 (`self.ConsistentMeshSizes`)) 1))
        (bind _returnvalue_3 (* _index _eachsectionlength_2))
        (set `self.DistanceStart` _returnvalue_3)
        (set `self.DistanceEnd` (+ _returnvalue_3 _eachsectionlength_2))
        (bind _returnvalue_4 (`AddComponent|NODE_AddSplineMeshComponent-1`))
        (bind _output_get_3 (set `self.MeshPart` _returnvalue_4))
        (`StaticMeshComponent.SetStaticMesh` _output_get_3 (`self.StaticMesh`))
        (`SplineMeshComponent.SetStartAndEnd` _output_get_3 (`SplineComponent.GetLocationAtDistanceAlongSpline` _spline _distancestart "Local") (`KismetMathLibrary.ClampVectorSize` (`SplineComponent.GetTangentAtDistanceAlongSpline` _spline _distancestart "Local") 0.0 _eachsectionlength) (`SplineComponent.GetLocationAtDistanceAlongSpline` _spline _distanceend "Local") (`KismetMathLibrary.ClampVectorSize` (`SplineComponent.GetTangentAtDistanceAlongSpline` _spline _distanceend "Local") 0.0 _eachsectionlength) true)
        (`PrimitiveComponent.SetCollisionEnabled` _output_get_3 (`self.CollisionType`))))))