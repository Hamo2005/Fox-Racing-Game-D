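; AI-driven vehicle that steers itself toward points on the level's TrackSpline1 actor.
; Each Tick it scans the spline points, replacing its stored nearest location with any closer one to set the wanted location.
; Steering maps the world look-at yaw to that target, without subtracting vehicle heading.
; Throttle is full except at high steering, where it equals the steering magnitude; both feed AIForward and AITurnRight.
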(event `self.ReceiveTick`
  (params (DeltaSeconds :type "Float (single-precision)"))
  (`parent.ReceiveTick` DeltaSeconds)
  (`self.Update Wanted Location`)
  (`self.AI_Forward` (`self.Get Throttle Input`))
  (`self.AI_Turn_Right` (`self.Get Steering Input`)))

(fn `Get Steering Input`
  (returns (`Steering Input` :type "Float (double-precision)"))
  (bind (_returnvalue_roll _returnvalue_pitch _returnvalue_yaw) (`KismetMathLibrary.BreakRotator` (`KismetMathLibrary.FindLookAtRotation` (`self.K2_GetActorLocation`) (`self.Wanted Location`))))
  ;[1 1 1] Get Steering Input
  (return (`KismetMathLibrary.MapRangeClamped` _returnvalue_yaw -180.0 180.0 -1.0 1.0)))

(fn `Get Throttle Input`
  (returns (NewParam :type "Float (double-precision)"))
  (bind _steering_input (`self.Get Steering Input`))
  ;[1 1 1] Get Throttle Input
  (return (select `bool` (or (> _steering_input 0.7) (< _steering_input -0.7)) :`false` 1.0 :`true` (`KismetMathLibrary.Abs` _steering_input))))

(fn `Update Wanted Location`
  (bind _returnvalue (`self.K2_GetActorLocation`))
  ;[1 1 1] Update Wanted Location
  (bind _returnvalue_2 (`GameplayStatics.GetActorOfClass` "/Game/Blueprints/Actors/SplineMeshes/TrackSpline1.TrackSpline1_C"))
  (bind _spline (`/Game/Blueprints/Actors/SplineMeshes/TrackSpline1.Spline` _returnvalue_2))
  (for _index (range (`SplineComponent.GetNumberOfSplinePoints` _spline))
    (bind _returnvalue_3 (`SplineComponent.GetLocationAtSplinePoint` _spline _index "World"))
    (if (and (> (- (`KismetMathLibrary.Vector_Distance` _returnvalue (`self.Nearest Location`)) (`KismetMathLibrary.Vector_Distance` _returnvalue _returnvalue_3)) 0.0) (`KismetMathLibrary.NotEqualExactly_VectorVector` (`self.Wanted Location`) _returnvalue_3))
      (set `self.Nearest Location` _returnvalue_3)))
  (set `self.Wanted Location` (`self.Nearest Location`)))

(fn `UserConstructionScript`
  (`parent.UserConstructionScript`))