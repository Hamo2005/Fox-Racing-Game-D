(event `self.ReceiveBeginPlay`
  (`self.Start Countdown`))

(event `Start Countdown`
  (`KismetSystemLibrary.PrintString` "Starting Countdown")
  (`KismetSystemLibrary.Delay` (`self.StartCountdown`))
  (`self.Game Start`))

(event `Game Start`
  (`KismetSystemLibrary.PrintString` "Starting Game")
  (bind _returnvalue (`KismetSystemLibrary.K2_SetTimerDelegate` (delegate `Lose-TimeOut`) (`self.TimeBetweenCheckpoints`)))
  (set `self.TimeRemainingTimer` _returnvalue))

(event `Lose-TimeOut`
  (`self.Game Finish` false))

(event `Win-CrossFinishLine`
  (`KismetSystemLibrary.K2_ClearAndInvalidateTimerHandle` (`self.TimeRemainingTimer`))
  (`self.Game Finish` false))

(event `Game Finish`
  (params (Win :type Boolean))
  (`KismetSystemLibrary.PrintString` (`KismetMathLibrary.SelectString` "You Win!" "You Lose!" Win)))

(fn `UserConstructionScript`)